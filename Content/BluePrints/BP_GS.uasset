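; BP_GS keeps the player's banana score in MPuntos.
; The score starts at zero on BeginPlay, rises by one when the player gets a banana and resets to zero when the player dies.
; Each change calls the OnPoint dispatcher with the current total, so listeners can react without polling.
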(event `OnPlayerDeath_Event`
  ;[1 0 0] Cuando el player muere
  (set `self.mPuntos` 0)
  (`self.OnPoint` (`self.mPuntos`)))

(event `OnPlayerGetBanana_Event`
  ;[1 0.9605 0] Cuando la banana toca al player
  (set `self.mPuntos` (+ (`self.mPuntos`) 1))
  (`self.OnPoint` (`self.mPuntos`)))

(event `self.ReceiveBeginPlay`
  ;[0 1 0] Empezar Partida
  (set `self.mPuntos` 0)
  (`self.OnPoint` (`self.mPuntos`)))

(fn `UserConstructionScript`)