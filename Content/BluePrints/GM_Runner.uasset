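; Runner game mode that runs a timed loop placing obstacle walls at random XZ positions around the player, plus bananas.
; It spawns BP_Obstaculo pairs until over eight exist, then recycles them by rotating index, drawing each banana from an object pool using the pair's coordinates.
; Recycling shortens the delay and re-arms the loop only while above the minimum.
; Player death restores the maximum delay and notifies BP_GS.
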(event `self.ReceiveBeginPlay`
  (set `self.mIndice` 0)
  (set `self.mTiempoActual` (`self.mTiempoIteracionMaximo`))
  (`KismetSystemLibrary.Delay` (`self.mTiempoActual`) :!label _label)
  (if (> (`KismetArrayLibrary.Array_Length` (`self.mObjetos`)) 8)
    ;[0.4891 0.3203 1] Reasignar posicion paredes y bananas
    (`|ExecutionSequence`
      (:`then_0`
        (bind (_outputpin _outputpin2) (`self.ReasignarPosicionPared`)))
      (:`then_1`
        (bind (_outputpin_2 _outputpin2_2) (`self.ReasignarPosicionPared`))
        (bind _returnvalue (`self.GetPositionToSpawnBanana` _outputpin_2 _outputpin2_2 _outputpin _outputpin2))
        (`/Game/ObjectPool/AC_ObjectPool.SpawnFromPool` (`self.AC_ObjectPool`) (`KismetMathLibrary.Conv_VectorToTransform` _returnvalue))
        ;[1 0.4714 0.1232] Incrementacion dificultad
        (if (> (`self.mTiempoActual`) (`self.mTiempoIteracionMinimo`))
          (set `self.mTiempoActual` (- (`self.mTiempoActual`) 0.2))
          (if (== (`self.mIndice`) 10)
            (set `self.mIndice` 0)
            (`self.OnReset`)
            (else
              (`self.OnReset`))))))
    (else
      ;[0.1264 0.8802 1] Spawn paredes y bananas
      (`|ExecutionSequence`
        (:`then_0`
          (bind (_returnvalue_x _returnvalue_z) (`self.SpawnPared`)))
        (:`then_1`
          (bind (_returnvalue_x_2 _returnvalue_z_2) (`self.SpawnPared`))
          (bind _returnvalue_2 (`self.GetPositionToSpawnBanana` _returnvalue_x_2 _returnvalue_z_2 _returnvalue_x _returnvalue_z))
          (`/Game/ObjectPool/AC_ObjectPool.SpawnFromPool` (`self.AC_ObjectPool`) (`KismetMathLibrary.Conv_VectorToTransform` _returnvalue_2))
          (`self.OnReset`))))))

(event `OnReset`
  (goto _label))

(event `OnPlayerDeath_Event`
  ;[1 0 0] Cuando el player muere
  (set `self.mTiempoActual` (`self.mTiempoIteracionMaximo`))
  (bind _asbp_gs (cast `/Game/BluePrints/BP_GS` (`GameplayStatics.GetGameState`)))
  (`/Game/BluePrints/BP_GS.OnPlayerDeath_Event` _asbp_gs))

(fn `GetPositionToSpawnBanana`
  (params (A :type "Float (double-precision)") (B :type "Float (double-precision)") (B2 :type "Float (double-precision)") (A2 :type "Float (double-precision)"))
  (returns (ReturnValue :type "Vector Structure"))
  (return (* (`KismetMathLibrary.Normal` (`KismetMathLibrary.MakeVector` (/ (+ A B2) 2.0) 0.0 (/ (+ A2 B) 2.0)) 0.0) (`self.mRangoPosicion`))))

(fn `ReasignarPosicionPared`
  (returns (OutputPin :type "Float (double-precision)") (OutputPin2 :type "Float (double-precision)"))
  (bind (_returnvalue_x _returnvalue_y) (`KismetMathLibrary.BreakVector` (`KismetMathLibrary.Vector_Normal2D` (`KismetMathLibrary.Conv_Vector2DToVector` (`KismetMathLibrary.MakeVector2D` (`KismetMathLibrary.RandomFloatInRange` -1.0 1.0) (`KismetMathLibrary.RandomFloatInRange` -1.0 1.0))) 0.0)))
  (bind (_returnvalue_x_2 _returnvalue_y_2 _returnvalue_z) (`KismetMathLibrary.BreakVector` (* (`KismetMathLibrary.MakeVector` _returnvalue_x 1.0 _returnvalue_y) (`self.mRangoPosicion`))))
  (bind (_returnvalue_x_3 _returnvalue_y_3 _returnvalue_z_2) (`KismetMathLibrary.BreakVector` (+ (`self.K2_GetActorLocation` (`GameplayStatics.GetPlayerPawn` 0)) (`KismetMathLibrary.MakeVector` _returnvalue_x_2 0.0 _returnvalue_z))))
  (`self.K2_SetActorLocation` (`|GetArrayItem` (`self.mObjetos`) (`self.mIndice`)) (`KismetMathLibrary.MakeVector` _returnvalue_x_3 _returnvalue_y_3 _returnvalue_z_2) false false)
  (bind _asbp_obstaculo (cast `/Game/BluePrints/BP_Obstaculo` (`|GetArrayItem` (`self.mObjetos`) (`self.mIndice`))))
  (`/Game/BluePrints/BP_Obstaculo.Get Target Position` _asbp_obstaculo)
  (set `self.mIndice` (+ (`self.mIndice`) 1))
  (return _returnvalue_x_3 _returnvalue_z_2))

(fn `SpawnPared`
  (returns (ReturnValue_X :type "Float (double-precision)") (ReturnValue_Z :type "Float (double-precision)"))
  (bind (_returnvalue_x _returnvalue_y) (`KismetMathLibrary.BreakVector` (`KismetMathLibrary.Vector_Normal2D` (`KismetMathLibrary.Conv_Vector2DToVector` (`KismetMathLibrary.MakeVector2D` (`KismetMathLibrary.RandomFloatInRange` -1.0 1.0) (`KismetMathLibrary.RandomFloatInRange` -1.0 1.0))) 0.0)))
  (bind (_returnvalue_x_2 _returnvalue_y_2 _returnvalue_z) (`KismetMathLibrary.BreakVector` (* (`KismetMathLibrary.MakeVector` _returnvalue_x 1.0 _returnvalue_y) (`self.mRangoPosicion`))))
  (bind (_returnvalue_x_3 _returnvalue_y_3 _returnvalue_z_2) (`KismetMathLibrary.BreakVector` (+ (`self.K2_GetActorLocation` (`GameplayStatics.GetPlayerPawn` 0)) (`KismetMathLibrary.MakeVector` _returnvalue_x_2 0.0 _returnvalue_z))))
  (bind _returnvalue (`|SpawnActorFromClass` "/Game/BluePrints/BP_Obstaculo.BP_Obstaculo_C" (`KismetMathLibrary.Conv_VectorToTransform` (`KismetMathLibrary.MakeVector` _returnvalue_x_3 _returnvalue_y_3 _returnvalue_z_2)) "Undefined" "MultiplyWithRoot" null null))
  (`KismetArrayLibrary.Array_Add` (`self.mObjetos`) _returnvalue)
  (return _returnvalue_x_3 _returnvalue_z_2))

(fn `SpawnTrueBanana`
  (params (InLocation :type "Vector Structure"))
  (`|SpawnActorFromClass` "/Game/BluePrints/BP_Banana.BP_Banana_C" (`KismetMathLibrary.Conv_VectorToTransform` InLocation) "Undefined" "MultiplyWithRoot" null 8.0 null))

(fn `UserConstructionScript`)