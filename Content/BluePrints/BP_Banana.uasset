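; BP_Banana is a banana pickup that flies in a straight line toward the player and reports to BP_GS when a pawn touches it.
; Activation through SetInUse calls the parent, then aims once at the pawn found by GetActorOfClass; Tick moves it along that fixed direction without sweeping.
; Pawn overlap fires the game state's banana event and sets the actor out of use rather than destroying it.
; The lifetime-based destroy logic is disconnected.
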(event `self.SetInUse`
  (params (InUse :type Boolean))
  (`parent.SetInUse` InUse)
  (if InUse
    (`self.GetPlayerDirection`)
    (else
      (`KismetSystemLibrary.PrintString` "No va"))))

(event `self.ReceiveActorBeginOverlap`
  (params (OtherActor :type "Actor Object Reference"))
  (cast `Pawn` OtherActor)
  (bind _asbp_gs (cast `/Game/BluePrints/BP_GS` (`GameplayStatics.GetGameState`)))
  (`/Game/BluePrints/BP_GS.OnPlayerGetBanana_Event` _asbp_gs)
  (`self.SetInUse` false))

(event `self.ReceiveTick`
  (params (DeltaSeconds :type "Float (single-precision)"))
  (`|ExecutionSequence`
    (:`then_0`
      ;[0.269 1 0.3029] Move
      (`self.K2_AddActorWorldOffset` (* (* DeltaSeconds (`self.mVelocity`)) (`self.mDirection`))))))

(fn `GetPlayerDirection`
  (bind _returnvalue (`GameplayStatics.GetActorOfClass` "/Script/Engine.Pawn"))
  (set `self.mDirection` (`KismetMathLibrary.Normal` (- (`self.K2_GetActorLocation` _returnvalue) (`self.K2_GetActorLocation`)) 0.0)))

(fn `UserConstructionScript`)