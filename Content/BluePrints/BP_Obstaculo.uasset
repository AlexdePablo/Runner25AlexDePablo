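; BP_Obstaculo is a runner obstacle that calls OnPlayerDeathEvent on GM_Runner when it overlaps a Pawn.
; It aims at a Pawn's location on BeginPlay and moves along that fixed direction each Tick, without sweep.
; Whenever its timer exceeds MResetTimer, it teleports to a random positive X/Z offset from the Pawn, scaled by MRangoPosicion, then re-aims.
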(event `self.ReceiveActorBeginOverlap`
  (params (OtherActor :type "Actor Object Reference"))
  (cast `Pawn` OtherActor)
  (if true
    (bind _asgm_runner (cast `/Game/BluePrints/GM_Runner` (`GameplayStatics.GetGameMode`)))
    (`/Game/BluePrints/GM_Runner.OnPlayerDeath_Event` _asgm_runner)))

(event `self.ReceiveBeginPlay`
  (`self.Get Target Position`))

(event `self.ReceiveTick`
  (params (DeltaSeconds :type "Float (single-precision)"))
  (bind (_returnvalue_x _returnvalue_y) (`KismetMathLibrary.BreakVector` (`KismetMathLibrary.Vector_Normal2D` (`KismetMathLibrary.Conv_Vector2DToVector` (`KismetMathLibrary.MakeVector2D` (`KismetMathLibrary.RandomFloat`) (`KismetMathLibrary.RandomFloat`))) 0.0)))
  (bind (_returnvalue_x_2 _returnvalue_y_2 _returnvalue_z) (`KismetMathLibrary.BreakVector` (* (`KismetMathLibrary.MakeVector` _returnvalue_x 1.0 _returnvalue_y) (`self.mRangoPosicion`))))
  ;[0.269 1 0.3029] Move
  (`|ExecutionSequence`
    (:`then_0`
      (`self.K2_AddActorWorldOffset` (* (* DeltaSeconds (`self.mVelocity`)) (`self.Direction`))))
    (:`then_1`
      (bind _output_get (set `self.mTimer` (+ DeltaSeconds (`self.mTimer`))))
      (if (> _output_get (`self.mResetTimer`))
        (set `self.mTimer` 0.0)
        (bind _returnvalue (`GameplayStatics.GetActorOfClass` "/Script/Engine.Pawn"))
        (`self.K2_SetActorLocation` (+ (`self.K2_GetActorLocation` _returnvalue) (`KismetMathLibrary.MakeVector` _returnvalue_x_2 0.0 _returnvalue_z)))
        (`self.Get Target Position`)))))

(fn `Get Target Position`
  (bind _returnvalue (`GameplayStatics.GetActorOfClass` "/Script/Engine.Pawn"))
  (set `self.Direction` (`KismetMathLibrary.Normal` (- (`self.K2_GetActorLocation` _returnvalue) (`self.K2_GetActorLocation`)))))

(fn `UserConstructionScript`)