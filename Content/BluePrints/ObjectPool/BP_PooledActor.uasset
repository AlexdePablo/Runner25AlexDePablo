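; Base actor for an object pool that toggles between active and dormant instead of being spawned and destroyed.
; SetInUse switches collision, visibility and ticking together, and BeginPlay starts the actor dormant.
; On activation it restarts a time-to-live timer that calls ReturnToPool, which deactivates it again.
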(event `self.ReceiveBeginPlay`
  (`self.SetInUse` false))

(event `SetInUse`
  (params (InUse :type Boolean))
  (set `self.InUse` InUse)
  (`self.SetActorEnableCollision` InUse)
  (`self.SetActorHiddenInGame` (not InUse))
  (`KismetSystemLibrary.K2_ClearAndInvalidateTimerHandle` (`self.TimeToLiveTimer`))
  (`self.SetActorTickEnabled` InUse)
  (if InUse
    (bind _returnvalue (`KismetSystemLibrary.K2_SetTimerDelegate` (delegate `ReturnToPool`) (`self.TimeToLive`)))
    (set `self.TimeToLiveTimer` _returnvalue)))

(event `ReturnToPool`
  (`self.SetInUse` false))

(fn `UserConstructionScript`)